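; BP_Bullet is a projectile actor that flies in a straight line and destroys itself when it overlaps another actor.
; Tick passes delta time to MoveEvent, which offsets the location by Direction and Speed without sweeping or a movement component.
; Any actor overlap calls InpactEvent, which only destroys the bullet, with no filtering or damage.
; An author comment flags MoveEvent as a possibly unnecessary multicast.
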(event `InpactEvent`
  (`self.K2_DestroyActor`))

(event `self.ReceiveActorBeginOverlap`
  (params (OtherActor :type "Actor Object Reference"))
  (`self.InpactEvent`))

(event `MoveEvent`
  (params (DeltaTime :type "Float (double-precision)"))
  ;[1 1 1] Maybe useless multicast
  (`self.K2_SetActorLocation` (+ (* (`self.Direction`) (* DeltaTime (`self.Speed`))) (`self.K2_GetActorLocation`))))

(event `self.ReceiveTick`
  (params (DeltaSeconds :type "Float (single-precision)"))
  (`self.MoveEvent` DeltaSeconds))

(fn `UserConstructionScript`)