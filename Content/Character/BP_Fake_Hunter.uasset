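; Player character posing as a human hunter who can temporarily turn into a monster by toggling two meshes.
; Monster form enables PanicCollision, registering itself as the Monster on overlapped AI, until a Tick timer restores human form.
; A Tick-driven Idle/Walk/Attack state lets the monster damage AI and hunters gathered by a sphere overlap, with DoOnce gates.
; Overlapping BP_Weapon swaps shadow casting to the hidden form's mesh; input also drives dash and sprint.
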(event `self.ReceiveBeginPlay`
  ;[1 1 1] Begin Play
  (`PrimitiveComponent.SetCollisionEnabled` (`self.PanicCollision`) "NoCollision")
  (set `self.bJumps` false)
  (`self.SetHealth` 10.0))

(event `Key|C`
  (params (Key :type "Key Structure"))
  ;[1 1 1] Dash
  (:`Pressed`
    (`/Engine/EditorBlueprintResources/StandardMacros.DoOnce` false :!label _label
      (:`Completed`
        (`self.Dash`)
        (if (not (`self.CheckHumanity`))
          (`/Game/Character/NewShadow/ABP_Darkness.DashAnim` (cast `/Game/Character/NewShadow/ABP_Darkness` (`SkeletalMeshComponent.GetAnimInstance` (`self.SkeletalMesh`)) :!pure true)))
        (`KismetSystemLibrary.Delay` 1.0)
        (`self.ResetDash`)))))

(event `ResetDash`
  ;[1 1 1] Dash
  (goto _label :!via `Reset`))

(event `CheckAbilityDuration`
  (params (deltaTime :type "Float (double-precision)"))
  ;[1 1 1] Check Transform duration
  (if (not (`self.CheckHumanity`))
    (bind _output_get (set `self.CurrentTimeAbility` (+ deltaTime (`self.CurrentTimeAbility`))))
    (if (> _output_get (`self.Duration`))
      (`self.HumanTransform`)
      (set `self.CurrentTimeAbility` 0.0)
      (`PrimitiveComponent.SetCollisionEnabled` (`self.PanicCollision`) "NoCollision"))))

(event `CheckIfWalking`
  (bind (_returnvalue_x _returnvalue_y) (`KismetMathLibrary.BreakVector` (`self.GetVelocity`)))
  ;[1 1 1] Check Status
  (if (or (> _returnvalue_x 0.0) (> _returnvalue_y 0.0))
    (`self.StateMoving`)
    (else
      (`self.StateIdle`))))

(event `Key|LeftShift`
  (params (Key :type "Key Structure"))
  ;[1 1 1] Sprint
  (:`Pressed`
    (`self.Sprint`))
  (:`Released`
    (`self.StopSprint`)))

(event `HumanTransform`
  ;[1 1 1] Human Transform
  (`SceneComponent.SetHiddenInGame` (`self.SkeletalMesh`) true false)
  (`SceneComponent.SetHiddenInGame` (`self.Mesh`) false false)
  (set `self.bCanTransform` true))

(event `RunOnServer`
  ;[1 1 1] Run transform on server
  (`self.MonsterTransform`)
  (`PrimitiveComponent.SetCollisionEnabled` (`self.PanicCollision`) "QueryOnly"))

(event `self.PanicCollision.OnComponentBeginOverlap`
  (params (OverlappedComponent :type "PrimitiveComponent Object Reference") (OtherActor :type "Actor Object Reference") (OtherComp :type "PrimitiveComponent Object Reference") (OtherBodyIndex :type Integer) (bFromSweep :type Boolean) (SweepResult :type "HitResult Structure (by ref)"))
  (bind _asbp_ai (cast `/Game/Character/AI/BP_AI` OtherActor))
  (bind _ac (`/Game/Character/AI/BP_AI.AC` _asbp_ai))
  (`/Engine/EditorBlueprintResources/StandardMacros.IsValid` _ac
    (:`Is Valid`
      (set `/Game/Character/AI/ABP_CitizenController.Monster` self _ac))))

(event `MonsterTransform`
  ;[1 1 1] Monster Form
  (if (`self.bCanTransform`)
    (`SceneComponent.SetHiddenInGame` (`self.SkeletalMesh`) false false)
    (`SceneComponent.SetHiddenInGame` (`self.Mesh`) true false)
    (`/Game/Character/NewShadow/ABP_Darkness.ChangeMode` (cast `/Game/Character/NewShadow/ABP_Darkness` (`SkeletalMeshComponent.GetAnimInstance` (`self.SkeletalMesh`)) :!pure true))
    (set `self.bCanTransform` false)))

(event `InputAction|Transform`
  (params (Key :type "Key Structure"))
  ;[1 1 1] Press key to change mode
  (:`Pressed`
    (`self.RunOnServer`)))

(event `self.PanicCollision.OnComponentEndOverlap`
  (params (OverlappedComponent :type "PrimitiveComponent Object Reference") (OtherActor :type "Actor Object Reference") (OtherComp :type "PrimitiveComponent Object Reference") (OtherBodyIndex :type Integer))
  (bind _asbp_ai (cast `/Game/Character/AI/BP_AI` OtherActor))
  (bind _ac (`/Game/Character/AI/BP_AI.AC` _asbp_ai))
  (`/Engine/EditorBlueprintResources/StandardMacros.IsValid` _ac
    (:`Is Valid`
      (if (== (`/Game/Character/AI/ABP_CitizenController.Monster` _ac) self)
        (set `/Game/Character/AI/ABP_CitizenController.Monster` null _ac)))))

(event `self.ReceiveTick`
  (params (DeltaSeconds :type "Float (single-precision)"))
  (bind _returnvalue (<= (`KismetArrayLibrary.Array_Length` (`self.GetOverlappingActors` "/Game/Actors/BP_Weapon.BP_Weapon_C")) 0))
  (bind _returnvalue_2 (<= (`KismetArrayLibrary.Array_Length` (`self.GetOverlappingActors` "/Game/Actors/BP_Weapon.BP_Weapon_C")) 0))
  (`self.CheckAbilityDuration` DeltaSeconds)
  (if (`self.CheckHumanity`)
    (`PrimitiveComponent.SetCastShadow` (`self.Mesh`) _returnvalue_2)
    (`PrimitiveComponent.SetCastShadow` (`self.SkeletalMesh`) (not _returnvalue_2))
    (else
      (`PrimitiveComponent.SetCastShadow` (`self.SkeletalMesh`) _returnvalue)
      (`PrimitiveComponent.SetCastShadow` (`self.Mesh`) (not _returnvalue))))
  (if (not (`|EnumEquality` (`self.CurrentState`) "NewEnumerator2"))
    (`self.CheckIfWalking`))
  (switch `/Game/Enumerate/E_ShadowState` (`self.CurrentState`)
    (:`NewEnumerator2`
      ;[1 1 1] Hit enemy
      (`self.Attack`)
      (if (and (not (`self.CheckHumanity`)) (`|EnumEquality` (`self.CurrentState`) "NewEnumerator2"))
        (`/Engine/EditorBlueprintResources/StandardMacros.DoOnce` false :!label _label_2
          (:`Completed`
            (`self.DisableInput` (`GameplayStatics.GetPlayerController` 0))
            (for _array_element (`self.ToAttack`)
              (`GameplayStatics.ApplyDamage` _array_element 1.0 null self))))))))

(event `ResetAttack`
  ;[1 1 1] Hit enemy
  (`self.EnableInput` (`GameplayStatics.GetPlayerController` 0))
  (set `self.CurrentState` "NewEnumerator1")
  (`self.Reset`)
  (goto _label_2 :!via `Reset`))

(event `StateIdle`
  ;[1 1 1] Change state in Walk
  (set `self.CurrentState` "NewEnumerator1"))

(event `StateMoving`
  ;[1 1 1] Change state in Walk
  (set `self.CurrentState` "NewEnumerator0"))

(event `self.Sphere.OnComponentBeginOverlap`
  (params (OverlappedComponent :type "PrimitiveComponent Object Reference") (OtherActor :type "Actor Object Reference") (OtherComp :type "PrimitiveComponent Object Reference") (OtherBodyIndex :type Integer) (bFromSweep :type Boolean) (SweepResult :type "HitResult Structure (by ref)"))
  (cast `/Game/Character/AI/BP_AI` OtherActor
    (:`then`
      _)
    (:`CastFailed`
      (cast `/Game/Character/BP_Hunter` OtherActor)))
  (`KismetArrayLibrary.Array_Add` (`self.ToAttack`) OtherActor))

(event `self.Sphere.OnComponentEndOverlap`
  (params (OverlappedComponent :type "PrimitiveComponent Object Reference") (OtherActor :type "Actor Object Reference") (OtherComp :type "PrimitiveComponent Object Reference") (OtherBodyIndex :type Integer))
  (bind _toattack (`self.ToAttack`))
  (bind _returnvalue (`KismetArrayLibrary.Array_Find` _toattack OtherActor))
  (if (!= _returnvalue -1)
    (`KismetArrayLibrary.Array_Remove` _toattack _returnvalue)))

(event `StateAttack`
  ;[1 1 1] Change state in Attack (Server side)
  (set `self.CurrentState` "NewEnumerator2"))

(event `Attack`
  ;[1 1 1] Attack (Set State Attack on server and play animation)
  (`/Engine/EditorBlueprintResources/StandardMacros.DoOnce` false :!label _label_3
    (:`Completed`
      (`self.StateAttack`)
      (`/Game/Character/NewShadow/ABP_Darkness.Attack` (cast `/Game/Character/NewShadow/ABP_Darkness` (`SkeletalMeshComponent.GetAnimInstance` (`self.SkeletalMesh`)) :!pure true))
      (`self.DisableInput` (`GameplayStatics.GetPlayerController` 0)))))

(event `Reset`
  ;[1 1 1] Attack (Set State Attack on server and play animation)
  (goto _label_3 :!via `Reset`))

(event `Key|SpaceBar`
  (params (Key :type "Key Structure"))
  ;[1 1 1] Input Attack (Change the current state in Attack state)
  (:`Pressed`
    (if (not (`self.CheckHumanity`))
      (set `self.CurrentState` "NewEnumerator2"))))

(fn `CheckHumanity`
  (returns (IsHuman :type Boolean))
  (return (not (`SceneComponent.IsVisible` (`self.SkeletalMesh`)))))

(fn `UserConstructionScript`
  (`parent.UserConstructionScript`))