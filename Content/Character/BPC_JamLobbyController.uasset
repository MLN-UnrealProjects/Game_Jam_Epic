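; Lobby player controller that handles a player's monster preference and ready state before a match.
; Preference and ready events pass the controller's JamPlayerState and new value to LobbyGameMode, which sets the status.
; Every tick it has the game instance update players' monster status locally.
; On EndPlay it collapses the lobby HUD and in-lobby menu widgets.
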(event `SetMonsterPreferences`
  (params (InWantsToBeMonster :type Boolean))
  ;[1 1 1] Set wants to be monster status
  (bind _aslobby_game_mode (cast `LobbyGameMode` (`GameplayStatics.GetGameMode`)))
  (bind _asjam_player_state (cast `JamPlayerState` (`self.PlayerState`)))
  (`LobbyGameMode.SetWantsToBeMonster` _aslobby_game_mode _asjam_player_state InWantsToBeMonster))

(event `self.ReceiveTick`
  (params (DeltaSeconds :type "Float (single-precision)"))
  (bind _asbp_jam_instance (cast `/Game/BP_Jam_instance` (`GameplayStatics.GetGameInstance`)))
  (`JamGameInstance.LobbyUpdatePlayersMonsterStatusLocal` _asbp_jam_instance))

(event `SetReadyState`
  (params (InReadyState :type Boolean))
  ;[1 1 1] Set ready status
  (bind _aslobby_game_mode (cast `LobbyGameMode` (`GameplayStatics.GetGameMode`)))
  (bind _asjam_player_state (cast `JamPlayerState` (`self.PlayerState`)))
  (`LobbyGameMode.SetReadyStatus` _aslobby_game_mode _asjam_player_state InReadyState))

(event `self.ReceiveEndPlay`
  (params (EndPlayReason :type "EEndPlayReason Enum" :default "Destroyed"))
  (bind _returnvalue (`self.GetInLobbyMenuWidget`))
  (bind _returnvalue_2 (`self.GetLobbyHUDWidget`))
  ;[1 1 1] Remove widgets
  (`/Engine/EditorBlueprintResources/StandardMacros.IsValid` _returnvalue_2
    (:`Is Valid`
      (`Widget.SetVisibility` _returnvalue_2 "Collapsed"))
    (:`Is Not Valid`
      _))
  (`/Engine/EditorBlueprintResources/StandardMacros.IsValid` _returnvalue
    (:`Is Valid`
      (`Widget.SetVisibility` _returnvalue "Collapsed"))))

(fn `UserConstructionScript`)