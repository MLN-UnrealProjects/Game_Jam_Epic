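; BP_Weapon is a weapon actor with a spotlight and cone collision that run on a limited, draining duration.
; On BeginPlay it fills ammo and duration, then Tick uses a timer accumulator to count the duration down in steps.
; Each step keeps the light and cone collision on, disabling both when duration runs out.
; Tick also caches the sphere's location as the shot origin and polls the R key to set a reload flag.
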(event `self.ReceiveBeginPlay`
  (set `self.Ammo` (`self.MaxAmmo`))
  (set `self.CurrentDuration` (`self.MaxDuration`)))

(event `self.ReceiveTick`
  (params (DeltaSeconds :type "Float (single-precision)"))
  (bind _spotlight (`self.SpotLight`))
  (bind _cone (`self.Cone`))
  (set `self.BeginShoot` (`SceneComponent.K2_GetComponentLocation` (`self.Sphere`)))
  (if (`PlayerController.IsInputKeyDown` (`GameplayStatics.GetPlayerController` 0) "R")
    (set `self.Reload` true))
  (bind _output_get (set `self.CurrentTime` (+ DeltaSeconds (`self.CurrentTime`))))
  (if (and (> _output_get (`self.MaxTime`)) (> (`self.CurrentDuration`) 0))
    (set `self.CurrentDuration` (- (`self.CurrentDuration`) 1))
    (set `self.CurrentTime` 0.0)
    (if (<= (`self.CurrentDuration`) 0)
      (`SceneComponent.SetVisibility` _spotlight false true)
      (`PrimitiveComponent.SetCollisionEnabled` _cone "NoCollision")
      (elif (not (`SceneComponent.IsVisible` _spotlight))
        (`SceneComponent.SetVisibility` _spotlight true false)
        (`PrimitiveComponent.SetCollisionEnabled` _cone "QueryAndPhysics")))))

(fn `OnRep_CurrentDuration`)

(fn `UserConstructionScript`)