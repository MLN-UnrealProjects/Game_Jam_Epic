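; Player controller for a jam game that owns the in-game UI and can host a multiplayer session.
; After login, the local controller creates the HUD and adds it to the viewport, and pre-creates the in-game menu, which HideInGameMenu removes while restoring game-only input.
; CreateSession shows the game instance's loading screen, creates a session using its LAN setting, then opens Level01 as a listen server.
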(event `ClientPostLogin`
  (`self.SetupIngameUI`))

(event `CreateSession`
  (bind _asjam_instance (cast `/Game/Core/Jam_instance` (`GameplayStatics.GetGameInstance`) :!pure true))
  (`/Game/Core/Jam_instance.ShowLoadingScreen` _asjam_instance)
  (`CreateSessionCallbackProxy.CreateSession` self 4 (`/Game/Core/Jam_instance.Enable LAN` _asjam_instance)
    (:`OnSuccess`
      (`GameplayStatics.OpenLevel` "Level01" true "listen"))
    (:`OnFailure`
      (`KismetSystemLibrary.PrintString` "failure to create" true true (struct :`G` 0.66 :`B` 1.0 :`A` 1.0) 3.0))))

(fn `HideInGameMenu`
  (`Widget.RemoveFromParent` (`self.InGameMenuWidget`))
  (`WidgetBlueprintLibrary.SetInputMode_GameOnly` self))

(fn `SetupIngameUI`
  (if (`self.IsLocalPlayerController`)
    (bind _returnvalue (`|CreateWidget` "/Game/Widget/UI_HUD.UI_HUD_C" self))
    (bind _output_get (set `self.HUDWidget` _returnvalue))
    (`UserWidget.AddToViewport` _output_get 0)
    (bind _returnvalue_2 (`|CreateWidget` "/Game/Widget/UI_InGameMenu.UI_InGameMenu_C" self))
    (set `self.InGameMenuWidget` _returnvalue_2)))

(fn `UserConstructionScript`)