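; Citizen NPC character that tracks its possessing AI controller and handles its own death.
; When Dead is set, Tick triggers the death animation once through BP_Anim_NPC and destroys the actor three seconds later.
; A Reset event loops AIMoveTo toward CurrentTarget, but only itself and disconnected code call it.
; Target-point wandering, idle pauses and walk-speed changes are disconnected leftovers, leaving ChooseTarget and MoveToLocation empty.
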(event `self.ReceiveBeginPlay`
  ;[1 1 1] Find all target points
)

(event `ChooseTarget`
  ;[1 1 1] Change target
)

(event `self.ReceiveTick`
  (params (DeltaSeconds :type "Float (single-precision)"))
  (if (`self.bDead`)
    (`/Engine/EditorBlueprintResources/StandardMacros.DoOnce` false
      (:`Completed`
        (`/Game/Character/AI/NPC/BP_Anim_NPC.Dead` (cast `/Game/Character/AI/NPC/BP_Anim_NPC` (`SkeletalMeshComponent.GetAnimInstance` (`self.Mesh`)) :!pure true))
        (`KismetSystemLibrary.Delay` 3.0)
        (`self.K2_DestroyActor`)))))

(event `ResetIdleEvent`)

(event `MoveToLocation`)

(event `self.ReceivePossessed`
  (params (NewController :type "Controller Object Reference"))
  (bind _asabp_citizen_controller (cast `/Game/Character/AI/ABP_CitizenController` NewController))
  (set `self.AC` _asabp_citizen_controller))

(event `Reset`
  (bind _currenttarget (`self.CurrentTarget`))
  (`/Engine/EditorBlueprintResources/StandardMacros.DoOnce` false :!via `Reset`
    (:`Completed`
      (`AITask_MoveTo.AIMoveTo` (`AIBlueprintHelperLibrary.GetAIController` self) (`self.K2_GetActorLocation` _currenttarget) _currenttarget -1.0 "Default" "Enable" true false
        (:`OnMoveFinished`
          (`self.ChooseTarget`)
          (`self.Reset`))))))

(event `self.ReceiveUnpossessed`
  (params (OldController :type "Controller Object Reference"))
  (if (== OldController (`self.AC`))
    (set `self.AC` null)))

(fn `UserConstructionScript`)