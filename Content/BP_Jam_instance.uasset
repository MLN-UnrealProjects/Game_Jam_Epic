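; Game instance Blueprint that manages the multiplayer session lifecycle: create, join and destroy.
; Creating a session uses the configured connection limit and LAN setting, then opens the lobby as a listen server; joining from a server list shows a loading screen.
; Create, join and destroy failures raise an error dialog.
; Shutdown destroys any session active in Lobby or Playing status to avoid crashes.
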(event `self.ReceiveShutdown`
  (bind _returnvalue (`GameplayStatics.GetPlayerController` 0))
  ;[1 1 1] On Shutdown Make sure no session is ongoing (should avoid editor and maybe in game crashes under certain circumstances)
  (switch `EGameStatus` (`self.GameStatus`)
    (:`Playing`
      _)
    (:`Lobby`
      _))
  (`/Engine/EditorBlueprintResources/StandardMacros.IsValid` _returnvalue
    (:`Is Valid`
      (`DestroySessionCallbackProxy.DestroySession` _returnvalue))))

(event `self.DestroySession`
  ;[1 1 1] Destroy Session
  (`DestroySessionCallbackProxy.DestroySession` (`GameplayStatics.GetPlayerController` 0)
    (:`OnSuccess`
      (`KismetSystemLibrary.PrintString` "Destroyed/Logout success" true true (struct :`G` 0.66 :`B` 1.0 :`A` 1.0) 10.0))
    (:`OnFailure`
      (`self.ShowErrorDialog` "Failed to destroy session"))))

(event `self.CreateSession`
  ;[1 1 1] Create Session
  (`CreateSessionCallbackProxy.CreateSession` (`GameplayStatics.GetPlayerController` 0) (`self.MaxConnections`) (`self.bEnableLAN`)
    (:`OnSuccess`
      (`GameplayStatics.OpenLevel` (`self.LobbyName`) true "listen"))
    (:`OnFailure`
      (`self.ShowErrorDialog` "Failed to create session" true))))

(event `JoinFromServerListEvent`
  (params (SearchResult :type "BlueprintSessionResult Structure"))
  ;[1 1 1] Join Session
  (`self.ShowLoadingScreen`)
  (`JoinSessionCallbackProxy.JoinSession` (`GameplayStatics.GetPlayerController` 0) SearchResult
    (:`OnFailure`
      (`self.ShowErrorDialog` "Failed to join session" true))))