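; BP_Weapon is a weapon actor with projectile and ray firing events, both based on its Sphere component as the muzzle.
; Shoot spawns a BP_Bullet at the Sphere's location and sets its Direction to the Sphere's forward vector.
; Shoot_Ray only draws a persistent debug Visibility trace from the Sphere to 10 units along that vector from the actor's origin, leaving the hit result unused.
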(event `Shoot`
  (bind _returnvalue (`|SpawnActorFromClass` "/Game/Components/BP_Bullet.BP_Bullet_C" (`KismetMathLibrary.MakeTransform` (`SceneComponent.K2_GetComponentLocation` (`self.Sphere`))) "Undefined" "OverrideRootScale" null null))
  (set `/Game/Components/BP_Bullet.Direction` (`SceneComponent.GetForwardVector` (`self.Sphere`)) _returnvalue))

(event `self.ReceiveTick`
  (params (DeltaSeconds :type "Float (single-precision)")))

(event `Shoot_Ray`
  (`KismetSystemLibrary.LineTraceSingle` :`Start` (`SceneComponent.K2_GetComponentLocation` (`self.Sphere`)) :`End` (+ (* (`SceneComponent.GetForwardVector` (`self.Sphere`)) 10.0) (`self.K2_GetActorLocation`)) :`TraceChannel` "TraceTypeQuery1" :`DrawDebugType` "Persistent"))

(fn `UserConstructionScript`)