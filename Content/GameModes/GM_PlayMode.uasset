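; Game mode for a humans-versus-monsters match that spawns a battery spawner on BeginPlay and quits when Escape is held.
; Win and draw events relay the result to each BPC_HunterController in the game instance's server player list.
; SpawnCitizens places a random number of citizen NPCs at popped spawn points, assigning each a selected mesh, material and AnimBP.
; An alternative EQS-based citizen spawn is present, but its query is never run.
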(event `self.ReceiveBeginPlay`
  (`|SpawnActorFromClass` "/Game/Actors/BP_BatterySpawner.BP_BatterySpawner_C" (`KismetMathLibrary.MakeTransform` (0.0 0.0 0.0)) "AlwaysSpawn" "OverrideRootScale" null null))

(event `self.ReceiveTick`
  (params (DeltaSeconds :type "Float (single-precision)"))
  (bind _returnvalue (`GameplayStatics.GetPlayerController` 0))
  (`/Engine/EditorBlueprintResources/StandardMacros.IsValid` _returnvalue
    (:`Is Valid`
      (if (`PlayerController.IsInputKeyDown` _returnvalue "Escape")
        (`KismetSystemLibrary.QuitGame` null "Quit")))))

(event `self.HumansHaveWon`
  (for _array_element (`JamGameInstance.GetServerPlayerList` (cast `/Game/BP_Jam_instance` (`GameplayStatics.GetGameInstance`) :!pure true))
    (bind _asbpc_hunter_controller (cast `/Game/Character/BPC_HunterController` (`.PlayerController` (break `LobbyPlayerMonsterData` _array_element))))
    (`GamePlayerController.HumansWon` _asbpc_hunter_controller)))

(event `self.MonstersHaveWon`
  (for _array_element (`JamGameInstance.GetServerPlayerList` (cast `/Game/BP_Jam_instance` (`GameplayStatics.GetGameInstance`) :!pure true))
    (bind _asbpc_hunter_controller (cast `/Game/Character/BPC_HunterController` (`.PlayerController` (break `LobbyPlayerMonsterData` _array_element))))
    (`GamePlayerController.MonstersWon` _asbpc_hunter_controller)))

(event `self.DrawnGame`
  (for _array_element (`JamGameInstance.GetServerPlayerList` (cast `/Game/BP_Jam_instance` (`GameplayStatics.GetGameInstance`) :!pure true))
    (bind _asbpc_hunter_controller (cast `/Game/Character/BPC_HunterController` (`.PlayerController` (break `LobbyPlayerMonsterData` _array_element))))
    (`GamePlayerController.DrawnGame` _asbpc_hunter_controller)))

(event `self.SpawnCitizens`
  (bind _output_get (set `self.CitizenSpawnCount` (`KismetMathLibrary.RandomIntegerInRange` (`self.MinCitizenCount`) (`self.MaxCitizenCount`))))
  (for _ (range (+ _output_get 1))
    (bind _returnvalue (`self.PopSpawnPoint`))
    (bind _returnvalue_2 (`|SpawnActorFromClass` (`self.CitizenPawn`) (`self.GetTransform` _returnvalue) "AlwaysSpawn" "OverrideRootScale" null null))
    (`/Engine/EditorBlueprintResources/StandardMacros.IsValid` _returnvalue_2
      (:`Is Valid`
        (`self.SelectModelInfosNPC`)
        (`JamCharacter.SetJamSkelMesh` _returnvalue_2 (`self.GetSelectedMesh`) (`self.GetSelectedMaterial`) (`self.GetSelectedAnimBP`))))))

(event `SpawnCitizenQuery`
  (params (QueryInstance :type "EnvQueryInstanceBlueprintWrapper Object Reference") (QueryStatus :type "EEnvQueryStatus Enum" :default "Processing"))
  (bind _returnvalue (`EnvQueryInstanceBlueprintWrapper.GetResultsAsActors` QueryInstance))
  (bind _returnvalue_2 (`KismetArrayLibrary.Array_Length` _returnvalue))
  (switch `EEnvQueryStatus` QueryStatus
    (:`Processing`
      (`KismetSystemLibrary.PrintString` "Progressing"))
    (:`Success`
      (`/Engine/EditorBlueprintResources/StandardMacros.IsValid` QueryInstance
        (:`Is Valid`
          (if (!= _returnvalue_2 0)
            (bind _output_get (set `self.CitizenSpawnCount` (`KismetMathLibrary.RandomIntegerInRange` (`self.MinCitizenCount`) (`self.MaxCitizenCount`))))
            (for _ (range (+ _output_get 1))
              (`|SpawnActorFromClass` (`self.CitizenPawn`) (`self.GetTransform` (`|GetArrayItem` _returnvalue (`KismetMathLibrary.RandomIntegerInRange` 0 (- _returnvalue_2 1)))) "AdjustIfPossibleButDontSpawnIfColliding" "OverrideRootScale" null null))
            (else
              (`KismetSystemLibrary.PrintString` "Invalid spawn point" :!label _label))))
        (:`Is Not Valid`
          (goto _label))))
    (:`Failed`
      (`KismetSystemLibrary.PrintString` "Failed"))
    (:`Aborted`
      (`KismetSystemLibrary.PrintString` "Aborted"))
    (:`OwnerLost`
      (`KismetSystemLibrary.PrintString` "OwnerLost"))
    (:`MissingParam`
      (`KismetSystemLibrary.PrintString` "MissingParams"))))

(fn `UserConstructionScript`)