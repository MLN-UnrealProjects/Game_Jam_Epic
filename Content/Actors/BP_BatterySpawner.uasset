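; BP_BatterySpawner is an actor that spawns BP_Battery pickups inside a box volume up to a maximum count.
; Tick accumulates time while below the cap, then spawns at a random point in the box once the timer is exceeded.
; Colliding spawns are refused, leaving the timer unreset so it retries next tick and prints a debug string.
; The battery count only increments in this graph.
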(event `self.ReceiveTick`
  (params (DeltaSeconds :type "Float (single-precision)"))
  (bind _box (`self.Box`))
  (if (not (== (`self.CurrentBatteriesInScene`) (`self.MaxBatteriesInScene`)))
    (bind _output_get (set `self.CurrentTime` (+ DeltaSeconds (`self.CurrentTime`))))
    (if (and (> _output_get (`self.SpawnTimer`)) (< (`self.CurrentBatteriesInScene`) (`self.MaxBatteriesInScene`)))
      (bind _returnvalue (`|SpawnActorFromClass` "/Game/Actors/BP_Battery.BP_Battery_C" (`KismetMathLibrary.MakeTransform` (`KismetMathLibrary.RandomPointInBoundingBox` (`SceneComponent.K2_GetComponentLocation` _box) (`BoxComponent.GetScaledBoxExtent` _box))) "DontSpawnIfColliding" "OverrideRootScale" null null))
      (if (`KismetSystemLibrary.IsValid` _returnvalue)
        (set `self.CurrentBatteriesInScene` (+ 1 (`self.CurrentBatteriesInScene`)))
        (set `self.CurrentTime` 0.0)
        (else
          (`KismetSystemLibrary.PrintString` "banana"))))))

(fn `UserConstructionScript`)