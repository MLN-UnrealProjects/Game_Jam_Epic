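; Projectile actor that flies in a straight line and damages the characters it overlaps.
; Each tick, MoveEvent offsets the location by Direction, Speed and delta time, without sweeping.
; Overlap takes health from a BP_Fake_Hunter or marks a BP_AI dead, then destroys the bullet through InpactEvent; other actors are ignored.
; A BP_Hunter damage branch is left unconnected.
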(event `InpactEvent`
  ;[1 1 1] Collision Events
  (`self.K2_DestroyActor`))

(event `self.ReceiveActorBeginOverlap`
  (params (OtherActor :type "Actor Object Reference"))
  ;[1 1 1] Collision Events
  (bind _asbp_fake_hunter (cast `/Game/Character/BP_Fake_Hunter` OtherActor)
    (:`then`
      (`/Game/ThirdPersonBP/Blueprints/BP_BaseCharacter.SetHealth` _asbp_fake_hunter (- (`JamCharacter.Health` _asbp_fake_hunter) 1.0)))
    (:`CastFailed`
      (bind _asbp_ai (cast `/Game/Character/AI/BP_AI` OtherActor))
      (set `/Game/Character/AI/BP_AI.bDead` true _asbp_ai)))
  (`self.InpactEvent`))

(event `self.ReceiveTick`
  (params (DeltaSeconds :type "Float (single-precision)"))
  (`self.MoveEvent` DeltaSeconds))

(event `MoveEvent`
  (params (DeltaTime :type "Float (double-precision)"))
  ;[1 1 1] Maybe useless multicast
  (`self.K2_SetActorLocation` (+ (* (`self.Direction`) (* DeltaTime (`self.Speed`))) (`self.K2_GetActorLocation`))))

(fn `UserConstructionScript`)