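; BP_Hunter is the hunter character, with sprinting, health and an attached weapon.
; On BeginPlay it spawns BP_Weapon on the mesh's weapon socket and caches the battery spawner.
; Overlapping a battery refills the weapon's duration, destroys the pickup and decrements the spawner's count.
; Health is polled every Tick; at zero it destroys itself and weapon, handing the controller a spectator pawn spawned at BP_Fake_Hunter.
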(event `self.ReceiveBeginPlay`
  ;[1 1 1] BeginPlay
  (`self.SpawnWeaponClient`)
  (bind _outactors (`GameplayStatics.GetAllActorsOfClass` "/Game/Actors/BP_BatterySpawner.BP_BatterySpawner_C"))
  (set `self.BatterySpawner` (`|GetArrayItem` _outactors)))

(event `Key|LeftShift`
  (params (Key :type "Key Structure"))
  ;[1 1 1] Sprint
  (:`Pressed`
    (`self.Sprint`))
  (:`Released`
    (`self.StopSprint`)))

(event `CheckLife`
  ;[1 1 1] CheckLife And Destroy if 0
  (if (<= (`self.Health`) 0.0)
    (bind _outactors (`GameplayStatics.GetAllActorsOfClass` "/Game/Character/BP_Fake_Hunter.BP_Fake_Hunter_C"))
    (bind _returnvalue (`|SpawnActorFromClass` "/Script/Engine.SpectatorPawn" (`self.GetTransform` (`|GetArrayItem` _outactors)) "Undefined" "OverrideRootScale" null null))
    (`self.K2_DestroyActor` (`self.Weapon`))
    (`Controller.Possess` (`self.GetController`) _returnvalue)
    (`self.K2_DestroyActor`)))

(event `self.ReceiveTick`
  (params (DeltaSeconds :type "Float (single-precision)"))
  ;[1 1 1] CheckLife And Destroy if 0
  (`self.CheckLife`))

(event `self.CapsuleComponent.OnComponentBeginOverlap`
  (params (OverlappedComponent :type "PrimitiveComponent Object Reference") (OtherActor :type "Actor Object Reference") (OtherComp :type "PrimitiveComponent Object Reference") (OtherBodyIndex :type Integer) (bFromSweep :type Boolean) (SweepResult :type "HitResult Structure (by ref)"))
  (bind _batteryspawner (`self.BatterySpawner`))
  (bind _weapon (`self.Weapon`))
  ;[1 1 1] Check if hit a battery
  (cast `/Game/Actors/BP_Battery` OtherActor)
  (set `/Game/Actors/BP_Weapon.CurrentDuration` (`/Game/Actors/BP_Weapon.MaxDuration` _weapon) _weapon)
  (`self.K2_DestroyActor` OtherActor)
  (set `/Game/Actors/BP_BatterySpawner.CurrentBatteriesInScene` (- (`/Game/Actors/BP_BatterySpawner.CurrentBatteriesInScene` _batteryspawner) 1) _batteryspawner))

(event `SpawnWeaponClient`
  ;[1 1 1] SpawnWeapon
  (bind _returnvalue (`|SpawnActorFromClass` "/Game/Actors/BP_Weapon.BP_Weapon_C" (`KismetMathLibrary.MakeTransform` (0.0 0.0 0.0)) "AlwaysSpawn" "OverrideRootScale" null null))
  (`self.K2_AttachToComponent` _returnvalue (`self.Mesh`) "weaponSocket" "KeepRelative" "KeepRelative" "KeepRelative" false)
  (set `self.Weapon` _returnvalue))

(event `SpawnWeapon`
  (`self.SpawnWeaponClient`))

(fn `UserConstructionScript`
  (`parent.UserConstructionScript`)
  (`self.SetHealth` 3.0))