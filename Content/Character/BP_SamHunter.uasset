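; BP_SamHunter is a character that carries a weapon and picks up batteries to recharge a torch.
; On BeginPlay it spawns BP_Weapon on the mesh's flashlight socket and caches the first BP_BatterySpawner.
; Capsule overlap with a BP_Battery refills the torch duration, destroys the battery and decrements the spawner's count.
; The flashlight spawn that assigns Torch is disconnected, so nothing here sets that reference.
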(event `ReadyForSpawn`
  (bind _returnvalue (`|SpawnActorFromClass` "/Game/Actors/BP_Weapon.BP_Weapon_C" (`KismetMathLibrary.MakeTransform` (0.0 0.0 0.0)) "Undefined" "OverrideRootScale" self null))
  (`self.K2_AttachToComponent` _returnvalue (`self.Mesh`) "flashlightSocket" "KeepRelative" "KeepWorld" "KeepRelative" true)
  (set `self.Weapon` _returnvalue))

(event `Spawn`
  (`self.ReadyForSpawn`))

(event `self.ReceiveBeginPlay`
  (`self.Spawn`)
  (bind _outactors (`GameplayStatics.GetAllActorsOfClass` "/Game/Actors/BP_BatterySpawner.BP_BatterySpawner_C"))
  (set `self.BatterySpawner` (`|GetArrayItem` _outactors)))

(event `self.CapsuleComponent.OnComponentBeginOverlap`
  (params (OverlappedComponent :type "PrimitiveComponent Object Reference") (OtherActor :type "Actor Object Reference") (OtherComp :type "PrimitiveComponent Object Reference") (OtherBodyIndex :type Integer) (bFromSweep :type Boolean) (SweepResult :type "HitResult Structure (by ref)"))
  (bind _torch (`self.Torch`))
  (bind _batteryspawner (`self.BatterySpawner`))
  (cast `/Game/Actors/BP_Battery` OtherActor)
  (set `/Game/Actors/BP_Flashlight.CurrentDuration` (`/Game/Actors/BP_Flashlight.MaxDuration` _torch) _torch)
  (`self.K2_DestroyActor` OtherActor)
  (set `/Game/Actors/BP_BatterySpawner.CurrentBatteriesInScene` (- (`/Game/Actors/BP_BatterySpawner.CurrentBatteriesInScene` _batteryspawner) 1) _batteryspawner))

(fn `UserConstructionScript`
  (`parent.UserConstructionScript`))