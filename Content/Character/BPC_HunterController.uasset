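; Player controller for the hunter character that handles shooting and the game-over screen.
; While alive, the Attack input spawns a bullet at the weapon's muzzle and flags a reload when ammo runs out.
; The weapon reference is cached from the possessed BP_Hunter through a DoOnce on Tick.
; The end-game widget is created at BeginPlay and shown after a delay with UI-only input and a visible cursor.
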(event `self.ReceiveEndPlay`
  (params (EndPlayReason :type "EEndPlayReason Enum" :default "Destroyed"))
  (bind _endgamescreen (`self.EndGameScreen`))
  (`/Engine/EditorBlueprintResources/StandardMacros.IsValid` _endgamescreen
    (:`Is Valid`
      (`Widget.SetVisibility` _endgamescreen "Hidden"))))

(event `self.ReceiveBeginPlay`
  (`/Engine/EditorBlueprintResources/StandardMacros.IsValid` (`self.EndGameScreen`)
    (:`Is Not Valid`
      (bind _returnvalue (`|CreateWidget` "/Game/UI/WBP_EndGame.WBP_EndGame_C" self))
      (set `self.EndGameScreen` _returnvalue))))

(event `self.ActivateGameoverScreen`
  (bind _endgamescreen (`self.EndGameScreen`))
  (`KismetSystemLibrary.Delay` (`self.DelayBeforeEndGameMenu`))
  (if (not (`Widget.IsInViewport` _endgamescreen))
    (`UserWidget.AddToViewport` _endgamescreen 0))
  (`Widget.SetVisibility` _endgamescreen "Visible")
  (`WidgetBlueprintLibrary.SetInputMode_UIOnlyEx` self _endgamescreen)
  (set `self.bShowMouseCursor` true))

(event `Shoot`
  (bind _weapon (`self.Weapon`))
  (bind _weapon_2 (`self.Weapon`))
  (bind _beginshoot (`/Game/Actors/BP_Weapon.BeginShoot` _weapon))
  (bind (_returnvalue_location _returnvalue_rotation) (`KismetMathLibrary.BreakTransform` (`SceneComponent.K2_GetComponentToWorld` _beginshoot)))
  (`/Engine/EditorBlueprintResources/StandardMacros.IsValid` _weapon
    (:`Is Valid`
      (if (not (`/Game/Actors/BP_Weapon.Reload` _weapon))
        (bind _returnvalue (`|SpawnActorFromClass` "/Game/Actors/BP_Bullet.BP_Bullet_C" (`KismetMathLibrary.MakeTransform` _returnvalue_location _returnvalue_rotation) "AlwaysSpawn" "OverrideRootScale" null null))
        (set `/Game/Actors/BP_Bullet.Direction` (`SceneComponent.GetForwardVector` _beginshoot) _returnvalue)
        (bind _result (`/Engine/EditorBlueprintResources/StandardMacros.DecrementInt` (`/Game/Actors/BP_Weapon.Ammo` _weapon_2))
          (:`  `
            (if (== _result 0)
              (set `/Game/Actors/BP_Weapon.Reload` true _weapon_2))))))))

(event `self.ReceiveTick`
  (params (DeltaSeconds :type "Float (single-precision)"))
  (if (`self.IsAlive`)
    (`/Engine/EditorBlueprintResources/StandardMacros.DoOnce` false
      (:`Completed`
        (bind _asbp_hunter (cast `/Game/Character/BP_Hunter` (`self.K2_GetPawn`)))
        (set `self.Weapon` (`/Game/Character/BP_Hunter.Weapon` _asbp_hunter))))))

(event `InputAction|Attack`
  (params (Key :type "Key Structure"))
  (:`Pressed`
    (if (`self.IsAlive`)
      (`self.Shoot`))))

(fn `UserConstructionScript`)