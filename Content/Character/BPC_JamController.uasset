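; Player controller for a jam game that opens the in-game menu and drives the controlled pawn.
; Pressing P shows the in-game menu, provided the UI is initialized and the menu is collapsed.
; MoveForward and MoveRight axes feed scaled movement input along the pawn's forward and right vectors, marked as temporary debug movement to remove.
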(event `Key|P`
  (params (Key :type "Key Structure"))
  (:`Pressed`
    (if (`self.IsUIInitialized`)
      (if (`self.IsInGameMenuCollapsed`)
        (`self.ShowInGameMenu`)))))

(event `InputAxis|MoveForward`
  (params (AxisValue :type "Float (single-precision)"))
  (bind _returnvalue (`self.K2_GetPawn`))
  ;[1 1 1] DEBUG movement to remove
  (`/Engine/EditorBlueprintResources/StandardMacros.IsValid` _returnvalue
    (:`Is Valid`
      (`Pawn.AddMovementInput` _returnvalue (`self.GetActorForwardVector` _returnvalue) (* AxisValue 10.0) false))))

(event `InputAxis|MoveRight`
  (params (AxisValue :type "Float (single-precision)"))
  (bind _returnvalue (`self.K2_GetPawn`))
  ;[1 1 1] DEBUG movement to remove
  (`/Engine/EditorBlueprintResources/StandardMacros.IsValid` _returnvalue
    (:`Is Valid`
      (`Pawn.AddMovementInput` _returnvalue (`self.GetActorRightVector` _returnvalue) (* AxisValue 10.0) false))))

(fn `UserConstructionScript`)